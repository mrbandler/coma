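; BP_PawnSpawner populates a tile board with player and opponent pawns, apparently as starting setup for a two-sided board game.
; SpawnPawns filters the context's tiles by row, giving the first two rows to the player and the last two to the opponent.
; A shared Spawn helper places the pawn class at each tile's transform, applies that side's material, and returns the spawned actors as two separate arrays.
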(fn SpawnPawns
  (params (PawnContext :type S%20Spawn%20Pawns%20Context%20Structure) (Board%20Context :type S%20Board%20Generation%20Context%20Structure))
  (bind (_tiles _pawn _playermaterial _opponentmaterial) (Utilities|Struct|BreakS_SpawnPawnsContext PawnContext))
  (bind _rows (Utilities|Struct|BreakS_BoardGenerationContext Board%20Context))
  (bind _pawns (CallFunction|Spawn (CallFunction|FilterTiles _tiles (Utilities|Array|MakeArray 0 1)) _pawn _playermaterial))
  (LocalVariables|SetOutPlayerPawns _pawns)
  (bind _pawns_2 (CallFunction|Spawn (CallFunction|FilterTiles _tiles (Utilities|Array|MakeArray (- _rows 2) (- _rows 1))) _pawn _opponentmaterial))
  (LocalVariables|SetOutOpponentPawns _pawns_2)
  (return (LocalVariables|GetOutPlayerPawns) (LocalVariables|GetOutOpponentPawns)))

(fn FilterTiles
  (params (Tiles :type Array%20of%20BP%20Tile%20Object%20References) (Rows :type Array%20of%20Integers))
  (for _array_element Tiles
    (if (Utilities|Array|ContainsItem Rows (.Row (Utilities|Struct|BreakS_BoardCoordinates (Variables|/Coma/BlueprintExample/BP_Tile.BP_Tile_C|GetCoordinates _array_element))))
      (Utilities|Array|Add (LocalVariables|GetTempTiles) _array_element)))
  (return (LocalVariables|GetTempTiles)))

(fn Spawn
  (params (Tiles :type Array%20of%20BP%20Tile%20Object%20References) (Pawn :type BP%20Pawn%20Class%20Reference) (Material :type Material%20Instance%20Object%20Reference))
  (for _array_element Tiles
    (bind _returnvalue (Game|SpawnActorfromClass Pawn (Transformation|GetActorTransform _array_element) "Undefined" 0 0))
    (Rendering|Material|SetMaterial (Variables|/Coma/BlueprintExample/BP_Pawn.BP_Pawn_C|GetMesh _returnvalue) 0 Material)
    (Utilities|Array|Add (LocalVariables|GetOutPawns) _returnvalue))
  (return (LocalVariables|GetOutPawns)))