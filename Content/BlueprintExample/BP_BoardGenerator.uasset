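; Board generator component that spawns a grid of tile actors in a checkerboard pattern and returns them.
; GenerateBoard stores the context, converts each index to board coordinates, and spawns the context's tile class for each one.
; Locations come from row and column times tile spacing, offset by the owner's X and Y at zero height.
; Each tile's setup receives its coordinates and a black or white material chosen by parity.
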(fn GenerateBoard
  (params (Context :type S%20Board%20Generation%20Context%20Structure))
  (bind _outtiles (LocalVariables|GetOutTiles))
  (bind _output_get (Variables|Default|SetContext Context))
  (bind _result (Math|Integer|DecrementInt (* (.Columns (Utilities|Struct|BreakS_BoardGenerationContext _output_get)) (.Rows (Utilities|Struct|BreakS_BoardGenerationContext _output_get))))
    (:%20%20
      (for _index (range 0 _result)
        (bind _tile (CallFunction|CreateTile (CallFunction|GetBoardCoordinatesfromIndex _index (.Columns (Utilities|Struct|BreakS_BoardGenerationContext _output_get)))))
        (Utilities|Array|Add _outtiles _tile))
      (return _outtiles))))

(fn CreateTile
  (params (BoardCoordinates :type S%20Board%20Coordinates%20Structure))
  (bind _returnvalue (Game|SpawnActorfromClass (.Tile (Utilities|Struct|BreakS_BoardGenerationContext (Variables|Default|GetContext))) (CallFunction|TileTransform BoardCoordinates) "Undefined" 0 0))
  (Default|Setup _returnvalue (Utilities|Struct|MakeS_TileContext BoardCoordinates (CallFunction|CoordinatestoMaterial BoardCoordinates)))
  (return _returnvalue))

(fn TileTransform
  (params (BoardCoordinates :type S%20Board%20Coordinates%20Structure))
  (return (Math|Transform|MakeTransform (CallFunction|TileLocation BoardCoordinates))))

(fn TileLocation
  (params (Coordinates :type S%20Board%20Coordinates%20Structure))
  (bind (_row _column) (Utilities|Struct|BreakS_BoardCoordinates Coordinates))
  (bind _returnvalue (Components|GetOwner))
  (bind _context (Variables|Default|GetContext))
  (bind _tilespacing (Utilities|Struct|BreakS_BoardGenerationContext _context))
  (bind _returnvalue_2 (Transformation|GetActorTransform _returnvalue))
  (bind _location (Math|Transform|BreakTransform _returnvalue_2))
  (bind (_x _y) (Math|Vector|BreakVector _location))
  (return (Math|Vector|MakeVector (+ (Math|Conversions|ToFloat(Integer) (* _row _tilespacing)) _x) (+ (Math|Conversions|ToFloat(Integer) (* _column _tilespacing)) _y) 0.0)))

(fn CoordinatestoMaterial
  (params (Coordinates :type S%20Board%20Coordinates%20Structure))
  (bind (_row _column) (Utilities|Struct|BreakS_BoardCoordinates Coordinates))
  (bind _context (Variables|Default|GetContext))
  (bind (_columns _rows _tile _tilespacing _whitematerial _blackmaterial) (Utilities|Struct|BreakS_BoardGenerationContext _context))
  (if (== (Math|Integer|%(Integer) (+ _row (Math|Integer|%(Integer) _column 2)) 2) 0)
    (LocalVariables|SetOutMaterial _blackmaterial)
    (else
      (bind _output_get (LocalVariables|SetOutMaterial _whitematerial))))
  (return _output_get))