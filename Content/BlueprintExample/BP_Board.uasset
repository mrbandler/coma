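; BP_Board builds the game board and places the pawns on it.
; Generate asks BoardGenerator to create the board from BoardContext and stores the resulting tiles in Tiles.
; It then passes those tiles, the pawn type and the player and opponent materials in a context struct to PawnSpawner, along with BoardContext, to spawn pawns for both sides.
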(fn Generate
  (bind _tiles (Default|GenerateBoard (Variables|Coma|GetBoardGenerator) (Variables|Board|GetBoardContext)))
  (bind _output_get (Variables|Board|SetTiles _tiles))
  (Default|SpawnPawns (Variables|Coma|GetPawnSpawner) (Utilities|Struct|MakeS_SpawnPawnsContext _output_get (Variables|Board|GetPawn) (Variables|Board|GetPlayerMaterial) (Variables|Board|GetOpponentMaterial)) (Variables|Board|GetBoardContext)))